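; BP_Floaters is an actor that bobs up and down around its starting position, like a floating object.
; The construction script stores Box1's world location and randomizes the starting phase, so instances move out of sync.
; Each Tick advances the phase by Speed and sets the actor's relative location to that stored position plus a vertical sine offset scaled by Offset.
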(event EventTick
  (params (DeltaSeconds :type Float%20%28single-precision%29))
  (Variables|Default|SetTheta (+ (Variables|Default|GetTheta) (* DeltaSeconds (Variables|Game|GetSpeed) 1e+02)))
  (Transformation|SetActorRelativeLocation (+ (Math|Vector|MakeVector 0.0 0.0 (* (Variables|Game|GetOffset) (Math|Trig|Sin(Degrees) (+ (Variables|Default|GetTheta) (* DeltaSeconds (Variables|Game|GetSpeed) 1e+02))))) (Variables|Default|GetInitialPosition))))

(fn ConstructionScript
  (Variables|Default|SetInitialPosition (Transformation|GetWorldLocation (Variables|Default|GetBox1)))
  (Variables|Default|SetTheta (Math|Random|RandomFloatinRange 0.0 3.6e+02)))