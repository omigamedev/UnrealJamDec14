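; BP_GameHUD is the in-game HUD, showing a power-up row and the player's life bar.
; DrawHUD draws everything with immediate-mode canvas calls at fixed pixel positions.
; Green, red and gray cube icons carry hardcoded count labels that read no game state.
; The life bar layers a green fill over a white background, scaling its width by Life from the player's BP_TempChar, treated as a fraction.
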(event EventDrawHUD
  (params (SizeX :type Integer) (SizeY :type Integer))
  (HUD|DrawText "Power-ups" "(R=1.000000,G=1.000000,B=1.000000,A=1.000000)" 4e+01 3e+01 "/Engine/EngineFonts/RobotoDistanceField.RobotoDistanceField" 1.0 false)
  (HUD|DrawText "x10" "(R=1.000000,G=1.000000,B=1.000000,A=1.000000)" 2.5e+02 3e+01 "/Engine/EngineFonts/RobotoDistanceField.RobotoDistanceField" 1.0 false)
  (Canvas|DrawTexture "/Game/Textures/icon_cube_green.icon_cube_green" 2e+02 2e+01 5e+01 5e+01 0.0 0.0 1.0 1.0 "(R=1.000000,G=1.000000,B=1.000000,A=1.000000)")
  (HUD|DrawText "x10" "(R=1.000000,G=1.000000,B=1.000000,A=1.000000)" 4e+02 3e+01 "/Engine/EngineFonts/RobotoDistanceField.RobotoDistanceField" 1.0 false)
  (Canvas|DrawTexture "/Game/Textures/icon_cube_red.icon_cube_red" 3.5e+02 2e+01 5e+01 5e+01 0.0 0.0 1.0 1.0 "(R=1.000000,G=1.000000,B=1.000000,A=1.000000)")
  (HUD|DrawText "x10" "(R=1.000000,G=1.000000,B=1.000000,A=1.000000)" 5.5e+02 3e+01 "/Engine/EngineFonts/RobotoDistanceField.RobotoDistanceField" 1.0 false)
  (Canvas|DrawTexture "/Game/Textures/icon_cube_gray.icon_cube_gray" 5e+02 2e+01 5e+01 5e+01 0.0 0.0 1.0 1.0 "(R=1.000000,G=1.000000,B=1.000000,A=1.000000)")
  (HUD|DrawText "Life" "(R=1.000000,G=1.000000,B=1.000000,A=1.000000)" 8e+02 3e+01 "/Engine/EngineFonts/RobotoDistanceField.RobotoDistanceField" 1.0 false)
  (HUD|DrawRect "(R=1.000000,G=1.000000,B=1.000000,A=1.000000)" 8.5e+02 3e+01 2e+02 25.0)
  (bind _asbp_temp_char (Utilities|Casting|CastToBP_TempChar (Game|GetPlayerCharacter 0)))
  (HUD|DrawRect "(R=0.719953,G=1.000000,B=0.574207,A=1.000000)" 8.5e+02 3e+01 (* (Variables|/Game/Blueprints/BP_TempChar.BP_TempChar_C|GetLife _asbp_temp_char) 2e+02) 25.0))

(fn ConstructionScript)