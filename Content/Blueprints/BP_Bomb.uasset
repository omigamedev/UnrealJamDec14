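; BP_Bomb is a bomb that heats up when something overlaps its sphere, then goes off with a radial impulse.
; The overlap restarts a timeline that drives the Hotness parameter on a dynamic material instance created in that event.
; When the timeline finishes, RadialForce1 fires its impulse and an Activate call follows.
; The construction script also stores a dynamic material in BombMat, which the event graph never uses.
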(event OnComponentBeginOverlap(Sphere1)
  (params (OtherActor :type Actor%20Object%20Reference) (OtherComp :type Primitive%20Component%20Object%20Reference) (OtherBodyIndex :type Integer) (bFromSweep :type Boolean) (SweepResult :type Hit%20Result%20Structure%20%28by%20ref%29))
  (bind _returnvalue (Rendering|Material|CreateDynamicMaterialInstance 0 0 :!class /Script/Engine.PrimitiveComponent))
  (bind _heat (Timeline|Timeline_0 PlayFromStart)
    (:Update
      (Rendering|Material|SetScalarParameterValue _returnvalue "Hotness" _heat :!class /Script/Engine.MaterialInstanceDynamic))
    (:Finished
      (Class|RadialForceComponent|FireImpulse (Variables|Default|GetRadialForce1))
      (Components|Activation|Activate false))))

(fn ConstructionScript
  (bind _returnvalue (Rendering|Material|CreateDynamicMaterialInstance (Rendering|Material|GetMaterial (Variables|Default|GetStaticMesh1) 0) 0 :!class /Script/Engine.KismetMaterialLibrary))
  (Variables|Default|SetBombMat _returnvalue))